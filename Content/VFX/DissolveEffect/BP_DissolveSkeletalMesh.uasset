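; Actor that plays an animated dissolve effect on a skeletal mesh with a matching Niagara particle effect.
; On BeginPlay the AnimateValue timeline drives Alpha, calling SetParams on every update.
; SetParams pushes alpha, edge settings and the dissolve texture to both mesh materials and Niagara, calling CreateDynamicMaterialInstance per slot each time.
; The construction script also calls SetParams, applying the settings at construction.
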(event `self.ReceiveBeginPlay`
  (bind (_direction _value) (`Timeline|AnimateValue`)
    (:`Update`
      (set `self.Alpha` _value)
      (`self.Set Params` (`self.SkeletalMesh`) (`self.NS_DissolveSkeletalMesh`)))))

(event `Set Params`
  (params (Mesh :type "MeshComponent Object Reference") (Niagara :type "NiagaraComponent Object Reference"))
  (`MeshComponent.SetScalarParameterValueOnMaterials` Mesh "Alpha" (`self.Alpha`))
  (`MeshComponent.SetVectorParameterValueOnMaterials` Mesh "Edge Color" (`KismetMathLibrary.Conv_LinearColorToVector` (`self.EdgeColor`)))
  (`MeshComponent.SetScalarParameterValueOnMaterials` Mesh "Edge Power" (`self.EdgePower`))
  (`MeshComponent.SetScalarParameterValueOnMaterials` Mesh "Edge Width" (`self.EdgeWidth`))
  (`MeshComponent.SetScalarParameterValueOnMaterials` Mesh "Edge Inner Width" (`self.EdgeInnerWidth`))
  (`NiagaraComponent.SetVariableFloat` Niagara "InnerEdge" (`self.InnerEdge`))
  (`NiagaraComponent.SetVariableFloat` Niagara "OuterEdge" (`self.OuterEdge`))
  (`NiagaraComponent.SetVariableFloat` Niagara "Alpha" (`self.Alpha`))
  (`NiagaraComponent.SetVariableLinearColor` Niagara "Edge Color" (`self.EdgeColor`))
  (`NiagaraFunctionLibrary.SetTextureObject` Niagara "Dissolve Texture" (`self.Dissolve Texture`))
  (for (_array_element _array_index) (`MeshComponent.GetMaterials` Mesh)
    (bind _returnvalue (`PrimitiveComponent.CreateDynamicMaterialInstance` Mesh _array_index _array_element "None"))
    (`MaterialInstanceDynamic.SetTextureParameterValue` _returnvalue "Dissolve Texture" (`self.Dissolve Texture`))))

(fn `UserConstructionScript`
  (`self.Set Params` (`self.SkeletalMesh`) (`self.NS_DissolveSkeletalMesh`)))