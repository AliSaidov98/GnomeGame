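; Actor that plays an animated dissolve effect on a static mesh, paired with a Niagara particle system.
; On BeginPlay, the AnimateValue timeline drives Alpha and calls SetParams on every update.
; SetParams pushes alpha, edge and dissolve texture settings to both mesh materials and Niagara, creating dynamic material instances for the texture on each call.
; The construction script repeats the same logic, applying the settings at construction.
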(event `self.ReceiveBeginPlay`
  (bind (_direction _value) (`Timeline|AnimateValue`)
    (:`Update`
      (set `self.Alpha` _value)
      (`self.Set Params`))))

(event `Set Params`
  (`MeshComponent.SetScalarParameterValueOnMaterials` (`self.StaticMesh`) "Alpha" (`self.Alpha`))
  (`MeshComponent.SetVectorParameterValueOnMaterials` (`self.StaticMesh`) "Edge Color" (`KismetMathLibrary.Conv_LinearColorToVector` (`self.EdgeColor`)))
  (`MeshComponent.SetScalarParameterValueOnMaterials` (`self.StaticMesh`) "Edge Power" (`self.EdgePower`))
  (`MeshComponent.SetScalarParameterValueOnMaterials` (`self.StaticMesh`) "Edge Width" (`self.EdgeWidth`))
  (`NiagaraComponent.SetVariableFloat` (`self.NS_DissolveMain`) "InnerEdge" (`self.InnerEdge`))
  (`NiagaraComponent.SetVariableFloat` (`self.NS_DissolveMain`) "OuterEdge" (`self.OuterEdge`))
  (`NiagaraComponent.SetVariableFloat` (`self.NS_DissolveMain`) "Alpha" (`self.Alpha`))
  (`NiagaraComponent.SetVariableLinearColor` (`self.NS_DissolveMain`) "Edge Color" (`self.EdgeColor`))
  (`NiagaraFunctionLibrary.SetTextureObject` (`self.NS_DissolveMain`) "Dissolve Texture" (`self.Dissolve Texture`))
  (for (_array_element _array_index) (`MeshComponent.GetMaterials` (`self.StaticMesh`))
    (bind _returnvalue (`PrimitiveComponent.CreateDynamicMaterialInstance` (`self.StaticMesh`) _array_index _array_element "None"))
    (`MaterialInstanceDynamic.SetTextureParameterValue` _returnvalue "Dissolve Texture" (`self.Dissolve Texture`))))

(fn `UserConstructionScript`
  (`MeshComponent.SetScalarParameterValueOnMaterials` (`self.StaticMesh`) "Alpha" (`self.Alpha`))
  (`MeshComponent.SetVectorParameterValueOnMaterials` (`self.StaticMesh`) "Edge Color" (`KismetMathLibrary.Conv_LinearColorToVector` (`self.EdgeColor`)))
  (`MeshComponent.SetScalarParameterValueOnMaterials` (`self.StaticMesh`) "Edge Power" (`self.EdgePower`))
  (`MeshComponent.SetScalarParameterValueOnMaterials` (`self.StaticMesh`) "Edge Width" (`self.EdgeWidth`))
  (`NiagaraComponent.SetVariableFloat` (`self.NS_DissolveMain`) "InnerEdge" (`self.InnerEdge`))
  (`NiagaraComponent.SetVariableFloat` (`self.NS_DissolveMain`) "OuterEdge" (`self.OuterEdge`))
  (`NiagaraComponent.SetVariableFloat` (`self.NS_DissolveMain`) "Alpha" (`self.Alpha`))
  (`NiagaraComponent.SetVariableLinearColor` (`self.NS_DissolveMain`) "Edge Color" (`self.EdgeColor`))
  (`NiagaraFunctionLibrary.SetTextureObject` (`self.NS_DissolveMain`) "Dissolve Texture" (`self.Dissolve Texture`))
  (for (_array_element _array_index) (`MeshComponent.GetMaterials` (`self.StaticMesh`))
    (bind _returnvalue (`PrimitiveComponent.CreateDynamicMaterialInstance` (`self.StaticMesh`) _array_index _array_element "None"))
    (`MaterialInstanceDynamic.SetTextureParameterValue` _returnvalue "Dissolve Texture" (`self.Dissolve Texture`))))